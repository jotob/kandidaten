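; Actor that applies a brightness value to post-process gamma, apparently as a screen brightness control.
; Each Tick, after a validity check, it refreshes Bright and linearly maps it into a narrow gamma range around neutral.
; The result fills all four channels of the Gamma vector and is written back into PostProcess settings every frame rather than only on change.
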(event `self.ReceiveTick`
  (params (DeltaSeconds :type "Float (single-precision)"))
  (bind _returnvalue (`KismetMathLibrary.Lerp` 0.9 1.2 (`self.bright`)))
  (`/Engine/EditorBlueprintResources/StandardMacros.IsValid` null
    (:`Is Valid`
      (set `self.bright` (`self.bright`))
      (bind _structout (setmembers `PostProcessSettings` :`StructRef` (`PostProcessComponent.Settings` (`self.Post Process`)) :`ColorGamma` (`KismetMathLibrary.MakeVector4` _returnvalue _returnvalue _returnvalue _returnvalue)))
      (set `PostProcessComponent.Settings` _structout (`self.Post Process`)))))

(fn `UserConstructionScript`)