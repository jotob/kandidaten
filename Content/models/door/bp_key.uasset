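; Key pickup Blueprint that gives the first-person character a key of a configurable type.
; The construction script picks the key mesh from KeyType, so each placed instance shows its matching model.
; On overlap with a FirstPersonCharacter, it adds KeyType to that character's OwendKeys collection, destroys itself and plays a 2D pickup sound.
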(event `self.overlap.OnComponentBeginOverlap`
  (params (OverlappedComponent :type "PrimitiveComponent Object Reference") (OtherActor :type "Actor Object Reference") (OtherComp :type "PrimitiveComponent Object Reference") (OtherBodyIndex :type Integer) (bFromSweep :type Boolean) (SweepResult :type "HitResult Structure (by ref)"))
  (bind _asfirst_person_character (cast `/Game/FirstPersonBP/Blueprints/FirstPersonCharacter` OtherActor))
  (`KismetArrayLibrary.Array_Add` (`/Game/FirstPersonBP/Blueprints/FirstPersonCharacter.owendKeys` _asfirst_person_character) (`self.keyType`))
  (`self.K2_DestroyActor`)
  (`GameplayStatics.PlaySound2D` "/Game/sund/key.key" 1.0 1.0 0.0 null null))

(fn `UserConstructionScript`
  (`StaticMeshComponent.SetStaticMesh` (`self.key`) (select `/Game/models/door/EKeyType` (`self.keyType`) :`NewEnumerator1` "/Game/models/key905.key905" :`NewEnumerator2` "/Game/models/key910.key910" :`NewEnumerator3` "/Game/models/key912.key912" :`NewEnumerator5` "/Game/models/key930.key930" :`NewEnumerator4` "/Game/models/key962.key962" :`NewEnumerator6` "/Game/models/key969.key969" :!type "StaticMesh Object Reference")))