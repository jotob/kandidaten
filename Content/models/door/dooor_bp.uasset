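; Interactive door that the player toggles with the openDoor input while the first-person character is inside its Interaction volume.
; It enables input for player 0 on BeginPlay, and the volume's overlap events open and close a Gate that filters presses.
; A FlipFlop alternates between the Dooranim and Clos timelines, both played from start, whose tracks lerp the handle's roll and the door's yaw between closed and open angles.
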(event `self.ReceiveBeginPlay`
  (`self.EnableInput` (`GameplayStatics.GetPlayerController` 0)))

(event `InputAction|openDoor`
  (params (Key :type "Key Structure"))
  (:`Pressed`
    (`/Engine/EditorBlueprintResources/StandardMacros.Gate` true :!label _label
      (:`Exit`
        (`/Engine/EditorBlueprintResources/StandardMacros.FlipFlop`
          (:`A`
            (bind (_direction _door_handle _door) (`Timeline|dooranim` :!via `PlayFromStart`)
              (:`Update`
                (`SceneComponent.K2_SetRelativeRotation` (`self.handle`) (`KismetMathLibrary.MakeRotator` (`KismetMathLibrary.Lerp` (`self.handle closed`) (`self.handle open`) _door_handle)) false false)
                (`SceneComponent.K2_SetRelativeRotation` (`self.door`) (`KismetMathLibrary.MakeRotator` 0.0 0.0 (`KismetMathLibrary.Lerp` (`self.closed`) (`self.open`) _door)) false false))))
          (:`B`
            (bind (_direction_2 _door_handle_2 _door_2) (`Timeline|clos` :!via `PlayFromStart`)
              (:`Update`
                (`SceneComponent.K2_SetRelativeRotation` (`self.handle`) (`KismetMathLibrary.MakeRotator` (`KismetMathLibrary.Lerp` (`self.handle closed`) (`self.handle open`) _door_handle_2)) false false)
                (`SceneComponent.K2_SetRelativeRotation` (`self.door`) (`KismetMathLibrary.MakeRotator` 0.0 0.0 (`KismetMathLibrary.Lerp` (`self.closed`) (`self.open`) _door_2)) false false)))))))))

(event `self.interaction.OnComponentBeginOverlap`
  (params (OverlappedComponent :type "PrimitiveComponent Object Reference") (OtherActor :type "Actor Object Reference") (OtherComp :type "PrimitiveComponent Object Reference") (OtherBodyIndex :type Integer) (bFromSweep :type Boolean) (SweepResult :type "HitResult Structure (by ref)"))
  (cast `/Game/FirstPersonBP/Blueprints/FirstPersonCharacter` OtherActor)
  (goto _label :!via `Open`))

(event `self.interaction.OnComponentEndOverlap`
  (params (OverlappedComponent :type "PrimitiveComponent Object Reference") (OtherActor :type "Actor Object Reference") (OtherComp :type "PrimitiveComponent Object Reference") (OtherBodyIndex :type Integer))
  (cast `/Game/FirstPersonBP/Blueprints/FirstPersonCharacter` OtherActor)
  (goto _label :!via `Close`))

(fn `UserConstructionScript`)